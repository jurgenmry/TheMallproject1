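; BP_WallClock is a wall clock actor that displays a time set by its Time variable.
; The construction script passes Time to SetTime, which rolls the OriginHours and OriginMins pivots to pose the hands.
; Time is in hours wrapped to a 12-hour dial, with the fractional part driving the minute hand.
; The event graph is empty, so the clock does not advance by itself during play.
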(fn `SetTime`
  (params (Time :type "Float (double-precision)"))
  (bind _returnvalue (mod Time 12.0))
  (`SceneComponent.K2_SetRelativeRotation` (`self.Origin_Hours`) (`KismetMathLibrary.MakeRotator` (* _returnvalue -30.0)) false false)
  (`SceneComponent.K2_SetRelativeRotation` (`self.Origin_Mins`) (`KismetMathLibrary.MakeRotator` (* (`KismetMathLibrary.Fraction` _returnvalue) -360.0)) false false))

(fn `UserConstructionScript`
  (`self.SetTime` (`self.Time`)))